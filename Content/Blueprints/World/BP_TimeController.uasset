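; World time controller Blueprint that sets the sun's rotation and keeps the sky sphere in sync with it.
; On BeginPlay it finds and caches the Directional Light and BP_Sky_Sphere, then refreshes the sky material.
; The UpdateTime event rotates the light to SunAngle, refreshes the sky and stores its SunHeight.
; Tick is unused, so updates happen only when UpdateTime is called.
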(event EventBeginPlay
  (bind _returnvalue (Actor|GetActorOfClass "/Script/Engine.DirectionalLight"))
  (Variables|Default|SetSun _returnvalue)
  (bind _returnvalue_2 (Actor|GetActorOfClass "/Engine/EngineSky/BP_Sky_Sphere.BP_Sky_Sphere_C"))
  (bind _output_get (Variables|Default|SetSkySphere _returnvalue_2))
  (Default|RefreshMaterial _returnvalue_2))

(event Collision|EventActorBeginOverlap
  (params (OtherActor :type Actor%20Object%20Reference)))

(event EventTick
  (params (DeltaSeconds :type Float%20%28single-precision%29)))

(event EventUpdateTime
  (bind _skysphere (Variables|Default|GetSkySphere))
  (Transformation|SetActorRotation (Variables|Default|GetSun) (Variables|Default|GetsunAngle))
  (Default|RefreshMaterial _skysphere)
  (Variables|Default|SetsunHeight (Variables|/Engine/EngineSky/BP_Sky_Sphere.BP_Sky_Sphere_C|GetSun%20height _skysphere)))

(fn ConstructionScript)