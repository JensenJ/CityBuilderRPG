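; Base player character with customisable body colour and name, a nameplate, and switchable first/third-person cameras.
; BeginPlay creates dynamic body and chest materials, sets a default name, hides the nameplate when locally controlled and runs the camera toggle, also bound to V.
; C opens or closes the CharacterEditor widget, switching input mode and cursor.
; SetBodyColour and SetName write RepNotify variables, whose OnRep functions refresh materials and nameplate.
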(event Custom|Set%20Body%20Colour
  (params (BodyColour :type Linear%20Color%20Structure))
  ;[1 1 1] Character Colouring
  (Variables|Default|SetBodyColour BodyColour))

(event Custom|OpenCharacterEditor
  (bind _returnvalue (Game|GetPlayerController 0))
  ;[1 1 1] Character Editor Widget Logic
  (bind _returnvalue_2 (UserInterface|CreateWidget "/Game/Blueprints/Character/CharacterEditor.CharacterEditor_C" _returnvalue))
  (UserInterface|Viewport|AddtoViewport _returnvalue_2 0)
  (Input|SetInputModeGameandUI _returnvalue 0 "DoNotLock" true)
  (Variables|/Script/Engine.PlayerController|SetbShowMouseCursor _returnvalue true)
  (Variables|Default|SetbEditingCharacter true))

(event Custom|CloseCharacterEditor
  (bind _returnvalue (Game|GetPlayerController 0))
  ;[1 1 1] Character Editor Widget Logic
  (bind _foundwidgets (Widget|GetAllWidgetsOfClass "/Game/Blueprints/Character/CharacterEditor.CharacterEditor_C" true))
  (Widget|RemovefromParent _foundwidgets)
  (Input|SetInputModeGameOnly _returnvalue)
  (Variables|/Script/Engine.PlayerController|SetbShowMouseCursor _returnvalue false)
  (Variables|Default|SetbEditingCharacter false))

(event Custom|Set%20Name
  (params (Name :type String))
  ;[1 1 1] Character Naming
  (Variables|Default|SetcharacterName Name))

(event EventBeginPlay
  (bind _mesh (Variables|Character|GetMesh))
  (bind _charactermovement (Variables|Character|GetCharacterMovement))
  (Utilities|FlowControl|Sequence
    (:then_0
      ;[1 1 1] Character Colouring
      (Utilities|FlowControl|Sequence
        (:then_0
          (bind _returnvalue (Rendering|Material|CreateDynamicMaterialInstance _mesh 0 "/Game/Mannequin/Character/Materials/M_UE4Man_Body.M_UE4Man_Body" "BodyMat" :!class /Script/Engine.PrimitiveComponent))
          (bind _output_get (Variables|Default|SetBodyMat _returnvalue))
          (Rendering|Material|SetMaterial _mesh 0 _output_get))
        (:then_1
          (bind _returnvalue_2 (Rendering|Material|CreateDynamicMaterialInstance _mesh 1 "/Game/Mannequin/Character/Materials/M_UE4Man_ChestLogo.M_UE4Man_ChestLogo" "ChestMat" :!class /Script/Engine.PrimitiveComponent))
          (bind _output_get_2 (Variables|Default|SetChestMat _returnvalue_2))
          (Rendering|Material|SetMaterial _mesh 1 _output_get_2))
        (:then_2
          (bind _returnvalue_3 (Rendering|Material|GetVectorParameterValue (Variables|Default|GetChestMat) "BodyColor" :!class /Script/Engine.MaterialInstanceDynamic))
          (Variables|Default|SetBodyColour _returnvalue_3))))
    (:then_1
      ;[1 1 1] Character Naming
      (Variables|Default|SetcharacterName "Player"))
    (:then_2
      ;[1 1 1] Nameplate Disable If Local
      (if (Pawn|IsLocallyControlled)
        (Rendering|SetVisibility (Variables|Default|GetNameplate) false false)))
    (:then_3
      ;[1 1 1] First / Third Person
      (if (Variables|Default|GetbThirdPerson)
        (Components|Activation|Activate (Variables|Default|GetFirstPersonCamera) false)
        (Components|Activation|Deactivate (Variables|Default|GetFollowCamera))
        (Variables|Default|SetbThirdPerson false)
        (Variables|Default|SetbUseControllerRotationYaw true)
        (Variables|/Script/Engine.CharacterMovementComponent|SetbOrientRotationToMovement _charactermovement false)
        (else
          (Components|Activation|Activate (Variables|Default|GetFollowCamera) false)
          (Components|Activation|Deactivate (Variables|Default|GetFirstPersonCamera))
          (Variables|Default|SetbThirdPerson true)
          (Variables|Default|SetbUseControllerRotationYaw false)
          (Variables|/Script/Engine.CharacterMovementComponent|SetbOrientRotationToMovement _charactermovement true))))))

(event Input|KeyboardEvents|C
  (params (Key :type Key%20Structure :default "None"))
  ;[1 1 1] Character Editor Widget Logic
  (:Released
    (if (Variables|Default|GetbEditingCharacter)
      (CallFunction|CloseCharacterEditor)
      (else
        (CallFunction|OpenCharacterEditor)))))

(event Input|KeyboardEvents|V
  (params (Key :type Key%20Structure :default "None"))
  (bind _charactermovement (Variables|Character|GetCharacterMovement))
  ;[1 1 1] First / Third Person
  (:Released
    (if (Variables|Default|GetbThirdPerson)
      (Components|Activation|Activate (Variables|Default|GetFirstPersonCamera) false)
      (Components|Activation|Deactivate (Variables|Default|GetFollowCamera))
      (Variables|Default|SetbThirdPerson false)
      (Variables|Default|SetbUseControllerRotationYaw true)
      (Variables|/Script/Engine.CharacterMovementComponent|SetbOrientRotationToMovement _charactermovement false)
      (else
        (Components|Activation|Activate (Variables|Default|GetFollowCamera) false)
        (Components|Activation|Deactivate (Variables|Default|GetFirstPersonCamera))
        (Variables|Default|SetbThirdPerson true)
        (Variables|Default|SetbUseControllerRotationYaw false)
        (Variables|/Script/Engine.CharacterMovementComponent|SetbOrientRotationToMovement _charactermovement true)))))

(fn ConstructionScript)

(fn OnRepBodyColour
  (bind _bodycolour (Variables|Default|GetBodyColour))
  (bind _bodymat (Variables|Default|GetBodyMat))
  (bind _chestmat (Variables|Default|GetChestMat))
  (Utilities|IsValid _bodymat
    (:Is%20Valid
      (Rendering|Material|SetVectorParameterValue _bodymat "BodyColor" _bodycolour :!class /Script/Engine.MaterialInstanceDynamic)
      (Utilities|IsValid _chestmat
        (:Is%20Valid
          (Rendering|Material|SetVectorParameterValue _chestmat "BodyColor" _bodycolour :!class /Script/Engine.MaterialInstanceDynamic)
          (bind _asname_plate (Utilities|Casting|CastToNamePlate (UserInterface|GetUserWidgetObject (Variables|Default|GetNameplate))))
          (Default|SetName _asname_plate (Variables|Default|GetcharacterName))
          (Default|SetColour _asname_plate (Variables|Default|GetBodyColour)))))))

(fn OnRepCharacterName
  (bind _asname_plate (Utilities|Casting|CastToNamePlate (UserInterface|GetUserWidgetObject (Variables|Default|GetNameplate))))
  (Default|SetName _asname_plate (Variables|Default|GetcharacterName))
  (Default|SetColour _asname_plate (Variables|Default|GetBodyColour)))