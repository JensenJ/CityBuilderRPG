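; Building placement ghost actor that follows the owning player's first-person camera aim and shows whether a spot is valid.
; Each tick a camera line trace positions it, snapping to the nearest snap point of a Building hit directly or found by a fallback box trace, otherwise optionally to a grid.
; A mesh-sized overlap box drives valid/invalid materials, with no trace hit counting as invalid.
; Events toggle both snapping modes and step the yaw rotation.
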(event Custom|SetValidPlacement
  (bind _staticmesh (Variables|Default|GetStaticMesh))
  ;[1 1 1] Setting Invalid / Valid Materials
  (for (_ _array_index) (Rendering|Material|GetMaterials _staticmesh)
    (Rendering|Material|SetMaterial _staticmesh _array_index "/Game/Materials/BuildingValid.BuildingValid"))
  (Variables|Default|SetbIsPlacementValid true))

(event Custom|SetInvalidPlacement
  (bind _staticmesh (Variables|Default|GetStaticMesh))
  ;[1 1 1] Setting Invalid / Valid Materials
  (for (_ _array_index) (Rendering|Material|GetMaterials _staticmesh)
    (Rendering|Material|SetMaterial _staticmesh _array_index "/Game/Materials/BuildingInvalid.BuildingInvalid"))
  (Variables|Default|SetbIsPlacementValid false))

(event Custom|RotateAntiClockwise
  ;[1 1 1] Line Tracing / Building Positioning
  (Variables|Default|SetRotationValue (+ (Variables|Default|GetRotationValue) (Variables|Default|GetrotationSnapAngle))))

(event Custom|RotateClockwise
  ;[1 1 1] Line Tracing / Building Positioning
  (Variables|Default|SetRotationValue (+ (* (Variables|Default|GetrotationSnapAngle) -1.0) (Variables|Default|GetRotationValue))))

(event Custom|ApplyRotation
  ;[1 1 1] Line Tracing / Building Positioning
  (Transformation|SetActorRotation (Math|Rotator|MakeRotator 0.0 0.0 (Variables|Default|GetRotationValue))))

(event Custom|ToggleBuildSnapping
  ;[1 1 1] Snap To Grid Toggle
  (Utilities|FlowControl|FlipFlop
    (:A
      (Variables|Default|SetbIsBuildSnappingEnabled false))
    (:B
      (Variables|Default|SetbIsBuildSnappingEnabled true))))

(event Custom|ToggleGridSnapping
  ;[1 1 1] Snap To Grid Toggle
  (Utilities|FlowControl|FlipFlop
    (:A
      (Variables|Default|SetbIsGridSnappingEnabled false))
    (:B
      (Variables|Default|SetbIsGridSnappingEnabled true))))

(event EventBeginPlay
  (bind _staticmesh (Variables|Default|GetStaticMesh))
  (bind _staticmesh_2 (Variables|Default|GetStaticMesh))
  (bind _overlapbox (Variables|Default|GetOverlapBox))
  (bind _boxextent (Collision|GetComponentBounds _staticmesh_2))
  ;[1 1 1] Building Setup
  (Components|StaticMesh|SetStaticMesh _staticmesh (Variables|Default|GetBuildingMesh))
  (for (_ _array_index) (Rendering|Material|GetMaterials _staticmesh)
    (Rendering|Material|SetMaterial _staticmesh _array_index "/Game/Materials/BuildingInvalid.BuildingInvalid"))
  (Variables|Default|SetbIsPlacementValid false)
  (Components|Box|SetBoxExtent _overlapbox (* (Math|Vector|MakeVector (.x _boxextent) (.y _boxextent) (.z _boxextent)) 0.9999) true)
  (Transformation|AddLocalOffset _overlapbox (Math|Vector|MakeVector 0.0 0.0 (.z _boxextent)) false false))

(event EventTick
  (params (DeltaSeconds :type Float%20%28single-precision%29))
  (bind _owningplayer (Variables|Default|GetOwningPlayer))
  (bind _bisplacementvalid (Variables|Default|GetbIsPlacementValid))
  (bind _bisgridsnappingenabled (Variables|Default|GetbIsGridSnappingEnabled))
  (bind _overlapbox (Variables|Default|GetOverlapBox))
  (bind _buildingrange (Variables|Default|GetBuildingRange))
  (bind _snapscale (Variables|Default|GetSnapScale))
  (bind _firstpersoncamera (Variables|/Game/Blueprints/Character/ThirdPersonCharacter.ThirdPersonCharacter_C|GetFirstPersonCamera _owningplayer))
  (bind _boxextent (Variables|/Script/Engine.BoxComponent|GetBoxExtent _overlapbox))
  (bind _returnvalue (Math|Vector|GetForwardVector _firstpersoncamera))
  (bind _returnvalue_2 (Transformation|GetWorldLocation _firstpersoncamera))
  (bind _returnvalue_3 (* _returnvalue _buildingrange))
  (bind _returnvalue_4 (+ _returnvalue_2 _returnvalue_3))
  ;[1 1 1] Line Tracing / Building Positioning
  (bind (_outhit _returnvalue_5) (Collision|LineTraceByChannel _returnvalue_2 _returnvalue_4 "TraceTypeQuery1" false 0 "None"))
  (if _returnvalue_5
    (if (.bSuccess (Utilities|Casting|CastToBuilding (.hitactor _outhit)))
      (if (Variables|Default|GetbIsBuildSnappingEnabled)
        (bind _output_get (Variables|Default|SetHitBuilding (.AsBuilding (Utilities|Casting|CastToBuilding (.hitactor _outhit)))))
        (bind _snappinglocation (CallFunction|FindClosestSnapPoint (.location _outhit) _output_get))
        (Transformation|SetActorLocation (+ _snappinglocation (Transformation|GetActorLocation (.AsBuilding (Utilities|Casting|CastToBuilding (.hitactor _outhit))))) false false)
        (else
          (if _bisgridsnappingenabled :!label _label
            (Transformation|SetActorLocation (Class|KismetMathLibrary|VectorSnappedtoGrid (.location _outhit) _snapscale) false false)
            (else
              (Transformation|SetActorLocation (.location _outhit) false false)))))
      (else
        (bind (_outhit_2 _returnvalue_6) (Class|KismetSystemLibrary|BoxTraceSingleforObjects (+ (.location _outhit) (Math|Vector|MakeVector 0.0 0.0 (.z _boxextent))) (+ (+ (.location _outhit) (Math|Vector|MakeVector 0.0 0.0 (.z _boxextent))) 0.1) (Math|Vector|MakeVector (.x _boxextent) (.y _boxextent) (.z _boxextent)) "0, 0, 0" (Utilities|Array|MakeArray "ObjectTypeQuery2") false 0 "None" true))
        (if _returnvalue_6
          (if (and (Variables|Default|GetbIsBuildSnappingEnabled) (.bSuccess (Utilities|Casting|CastToBuilding (.hitactor _outhit_2))))
            (bind _snappinglocation_2 (CallFunction|FindClosestSnapPoint (.location _outhit_2) (.AsBuilding (Utilities|Casting|CastToBuilding (.hitactor _outhit_2)))))
            (Transformation|SetActorLocation (+ _snappinglocation_2 (Transformation|GetActorLocation (.AsBuilding (Utilities|Casting|CastToBuilding (.hitactor _outhit_2))))) false false)
            (else
              (goto _label)))
          (else
            (goto _label)))))
    (CallFunction|ApplyRotation)
    ;[1 1 1] Condition Checking
    (if (not (Variables|Default|GetbHasOverlappingActors))
      (if (not _bisplacementvalid)
        (CallFunction|SetValidPlacement))
      (else
        (CallFunction|SetInvalidPlacement :!label _label_2)))
    (else
      (if _bisgridsnappingenabled
        (Transformation|SetActorLocation (Class|KismetMathLibrary|VectorSnappedtoGrid _returnvalue_4 _snapscale) false false)
        (else
          (Transformation|SetActorLocation _returnvalue_4 false false)))
      (CallFunction|ApplyRotation)
      (if _bisplacementvalid
        (goto _label_2)))))

(event Collision|EventActorBeginOverlap
  (params (OtherActor :type Actor%20Object%20Reference))
  ;[1 1 1] CollisionDetection
  (if (> (Utilities|Array|Length (Collision|GetOverlappingActors (Variables|Default|GetOverlapBox) "/Script/Engine.Actor" :!class /Script/Engine.PrimitiveComponent)) 0)
    (Variables|Default|SetbHasOverlappingActors true)))

(event Collision|EventActorEndOverlap
  (params (OtherActor :type Actor%20Object%20Reference))
  ;[1 1 1] CollisionDetection
  (if (== (Utilities|Array|Length (Collision|GetOverlappingActors (Variables|Default|GetOverlapBox) "/Script/Engine.Actor" :!class /Script/Engine.PrimitiveComponent)) 0)
    (Variables|Default|SetbHasOverlappingActors false)))

(fn ConstructionScript)

(fn FindClosestSnapPoint
  (params (HitLocation :type Vector) (HitBuilding :type Building%20Object%20Reference))
  (for (_array_element _array_index) (Variables|/Game/Blueprints/Building/Building.Building_C|GetSnapPositions HitBuilding)
    (if (== _array_index 0)
      (LocalVariables|SetClosestDistance (Math|Vector|VectorLength (- HitLocation (+ _array_element (Transformation|GetActorLocation HitBuilding)))) :!label _label)
      (LocalVariables|SetSnappingOffset _array_element)
      (elif (< (Math|Vector|VectorLength (- HitLocation (+ _array_element (Transformation|GetActorLocation HitBuilding)))) (LocalVariables|GetClosestDistance))
        (goto _label))))
  (return (* (LocalVariables|GetSnappingOffset) 2.0)))