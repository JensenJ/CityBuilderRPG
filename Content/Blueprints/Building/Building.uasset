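; Building actor that calculates its own snap points when play begins.
; BeginPlay shrinks the bounding box extent by 1% and rounds each axis up to whole 100-unit steps.
; From that it fills six offsets: four side centers, the actor origin and a top point, implying a bottom pivot.
; Long-lived debug spheres mark each offset added to the actor location, without applying rotation.
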(event EventBeginPlay
  (bind _boxextent (Collision|GetActorBounds false false))
  (bind _snappositions (Variables|Default|GetSnapPositions))
  (bind _returnvalue (* _boxextent 0.99))
  (bind _returnvalue_2 (/ _returnvalue 1e+02))
  ;[1 1 1] Calculate Actor Bounding Box
  (Variables|Default|SetBuildingBounds (* (Math|Vector|MakeVector (Math|Conversions|ToFloat(Integer) (Math|Float|Ceil (.x _returnvalue_2))) (Math|Conversions|ToFloat(Integer) (Math|Float|Ceil (.y _returnvalue_2))) (Math|Conversions|ToFloat(Integer) (Math|Float|Ceil (.z _returnvalue_2)))) 1e+02))
  ;[1 1 1] Calculate Snap Positions
  (Utilities|Array|SetArrayElem _snappositions 0 (Math|Vector|MakeVector (.x (Variables|Default|GetBuildingBounds)) 0.0 (.z (Variables|Default|GetBuildingBounds))))
  (Utilities|Array|SetArrayElem _snappositions 1 (Math|Vector|MakeVector (* (.x (Variables|Default|GetBuildingBounds)) -1.0) 0.0 (.z (Variables|Default|GetBuildingBounds))))
  (Utilities|Array|SetArrayElem _snappositions 2 (Math|Vector|MakeVector 0.0 (.y (Variables|Default|GetBuildingBounds)) (.z (Variables|Default|GetBuildingBounds))))
  (Utilities|Array|SetArrayElem _snappositions 3 (Math|Vector|MakeVector 0.0 (* (.y (Variables|Default|GetBuildingBounds)) -1.0) (.z (Variables|Default|GetBuildingBounds))))
  (Utilities|Array|SetArrayElem _snappositions 4 (Math|Vector|MakeVector 0.0 0.0 0.0))
  (Utilities|Array|SetArrayElem _snappositions 5 (Math|Vector|MakeVector 0.0 0.0 (* (.z (Variables|Default|GetBuildingBounds)) 2.0)))
  (for _array_element _snappositions
    (Rendering|Debug|DrawDebugSphere (+ _array_element (Transformation|GetActorLocation)) 5e+01 4 "(R=1.000000,G=1.000000,B=1.000000,A=1.000000)" 1e+03 1.0)))

(fn ConstructionScript)