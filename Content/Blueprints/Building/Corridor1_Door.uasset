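; Corridor door that opens automatically when a Pawn enters its trigger volume and closes when the last one leaves.
; Overlap events check the Pawns inside and use a DoorOpen flag to play the open or close skeletal mesh animation at a configurable rate.
; A reversal mid-animation starts the opposite animation at one minus the current position, which assumes one-second clips.
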(event OnComponentBeginOverlap(OpenCloseTriggerVolume)
  (params (OverlappedComponent :type Primitive%20Component%20Object%20Reference) (OtherActor :type Actor%20Object%20Reference) (OtherComp :type Primitive%20Component%20Object%20Reference) (OtherBodyIndex :type Integer) (bFromSweep :type Boolean) (SweepResult :type Hit%20Result%20Structure%20%28by%20ref%29))
  (bind _skeletalmesh (Variables|Default|GetSkeletalMesh))
  ;[1 1 1] Door Open / Close
  (if (> (Utilities|Array|Length (Collision|GetOverlappingActors (Variables|Default|GetOpenCloseTriggerVolume) "/Script/Engine.Pawn" :!class /Script/Engine.PrimitiveComponent)) 0)
    (if (not (Variables|Default|GetbDoorOpen))
      (bind _output_get (Variables|Default|SetcurrentPosition (Class|SkeletalMeshComponent|GetPosition _skeletalmesh)))
      (bind _output_get_2 (Variables|Default|SetbIsAnimating (Audio|Components|Audio|IsPlaying _skeletalmesh)))
      (Components|Animation|PlayAnimation _skeletalmesh "/Game/Models/FBXFiles/Corridor1/Corridor1_Door_Anim_Open.Corridor1_Door_Anim_Open" false)
      (Variables|Default|SetbDoorOpen true)
      (Components|Timeline|SetPlayRate _skeletalmesh (Variables|Default|GetanimationPlayRate))
      (if _output_get_2
        (Components|Animation|SetPosition _skeletalmesh (- 1.0 _output_get) true))
      (Variables|Default|SetcurrentPosition 0.0))))

(event OnComponentEndOverlap(OpenCloseTriggerVolume)
  (params (OverlappedComponent :type Primitive%20Component%20Object%20Reference) (OtherActor :type Actor%20Object%20Reference) (OtherComp :type Primitive%20Component%20Object%20Reference) (OtherBodyIndex :type Integer))
  (bind _skeletalmesh (Variables|Default|GetSkeletalMesh))
  ;[1 1 1] Door Open / Close
  (if (== (Utilities|Array|Length (Collision|GetOverlappingActors (Variables|Default|GetOpenCloseTriggerVolume) "/Script/Engine.Pawn" :!class /Script/Engine.PrimitiveComponent)) 0)
    (if (Variables|Default|GetbDoorOpen)
      (bind _output_get (Variables|Default|SetcurrentPosition (Class|SkeletalMeshComponent|GetPosition _skeletalmesh)))
      (bind _output_get_2 (Variables|Default|SetbIsAnimating (Audio|Components|Audio|IsPlaying _skeletalmesh)))
      (Components|Animation|PlayAnimation _skeletalmesh "/Game/Models/FBXFiles/Corridor1/Corridor1_Door_Anim_Close.Corridor1_Door_Anim_Close" false)
      (Variables|Default|SetbDoorOpen false)
      (Components|Timeline|SetPlayRate _skeletalmesh (Variables|Default|GetanimationPlayRate))
      (if _output_get_2
        (Components|Animation|SetPosition _skeletalmesh (- 1.0 _output_get) true))
      (Variables|Default|SetcurrentPosition 0.0))))

(fn ConstructionScript)