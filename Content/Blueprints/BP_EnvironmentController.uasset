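; Environment controller that drives the level's directional light sun and sky sphere.
; On BeginPlay it finds and caches the DirectionalLight and BP_Sky_Sphere actors, then refreshes the sky material.
; The UpdateEnvironment event applies the stored sun angle and intensity to the light, refreshes the sky, and copies back the sky sphere's sun height.
; Nothing runs on Tick, so later changes apply only when that event is called.
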(event EventBeginPlay
  (bind _returnvalue (Actor|GetActorOfClass "/Script/Engine.DirectionalLight"))
  (Variables|Default|SetSun _returnvalue)
  (bind _returnvalue_2 (Actor|GetActorOfClass "/Engine/EngineSky/BP_Sky_Sphere.BP_Sky_Sphere_C"))
  (bind _output_get (Variables|Default|SetSkysphere _returnvalue_2))
  (Default|RefreshMaterial _output_get))

(event Collision|EventActorBeginOverlap
  (params (OtherActor :type Actor%20Object%20Reference)))

(event EventTick
  (params (DeltaSeconds :type Float%20%28single-precision%29)))

(event EventUpdateEnvironment
  (bind _sun (Variables|Default|GetSun))
  (bind _skysphere (Variables|Default|GetSkysphere))
  (Transformation|SetActorRotation _sun (Variables|Default|GetsunAngle))
  (Rendering|Components|Light|SetIntensity (Variables|/Script/Engine.Light|GetLightComponent _sun) (Variables|Default|GetsunIntensity))
  (Default|RefreshMaterial _skysphere)
  (Variables|Default|SetsunHeight (Variables|/Engine/EngineSky/BP_Sky_Sphere.BP_Sky_Sphere_C|GetSun%20height _skysphere)))

(fn ConstructionScript)